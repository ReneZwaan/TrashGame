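; Space garbage actor in Big or Small variants that gets a random mesh, rotation and starting spin on BeginPlay, with scale set per type.
; Only Big pieces react to projectile hits, counting them and playing the GotHit timeline until a random hit limit is reached.
; At the limit the piece explodes with VFX and sound, spawns a cluster of Small instances of itself nearby, and destroys itself.
; An impulse toward the trash truck is left unconnected.
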(event `self.ReceiveBeginPlay`
  (`self.Random Mesh`)
  (set `self.MaxHitTime` (`KismetMathLibrary.RandomIntegerInRange` 3 5))
  (`self.K2_SetActorRotation` (`KismetMathLibrary.RandomRotator` false) true)
  (`PrimitiveComponent.AddTorqueInRadians` (`self.Mesh`) (* (`KismetMathLibrary.RandomUnitVector`) (* (`KismetMathLibrary.RandomFloat`) (`self.MaxStartTorque`))) "None" true))

(event `self.Mesh.OnComponentHit`
  (params (HitComponent :type "PrimitiveComponent Object Reference") (OtherActor :type "Actor Object Reference") (OtherComp :type "PrimitiveComponent Object Reference") (NormalImpulse :type "Vector Structure") (Hit :type "HitResult Structure (by ref)"))
  (bind (_returnvalue_x _returnvalue_y _returnvalue_z) (`KismetMathLibrary.BreakVector` (`self.K2_GetActorLocation`)))
  (cast `/Game/Assets/SpaceGun/BP_Projectile` OtherActor)
  (switch `/Game/Assets/SpaceGrabage/E_GrabageType` (`self.GrabageType`)
    (:`NewEnumerator0`
      (`/Engine/EditorBlueprintResources/StandardMacros.IncrementInt` (`self.GotHitTimes`)
        (:`  `
          (if (>= (`self.GotHitTimes`) (`self.MaxHitTime`))
            (`GameplayStatics.SpawnEmitterAtLocation` "/Game/GrenadePack/Particles/VFX_GrenadeEXP_air.VFX_GrenadeEXP_air" (`self.K2_GetActorLocation`) (struct) (20.0 20.0 20.0))
            (`GameplayStatics.SpawnSoundAtLocation` "/Game/Assets/Sound/explore_Cue.explore_Cue" (`self.K2_GetActorLocation`) (struct) 1.0 1.0 0.0 null null)
            (for _ (range 26)
              (`|SpawnActorFromClass` "BP_SpaceGrabage_C" (`KismetMathLibrary.MakeTransform` (`KismetMathLibrary.MakeVector` (`KismetMathLibrary.RandomFloatInRange` (+ _returnvalue_x -50.0) (+ _returnvalue_x 50.0)) (`KismetMathLibrary.RandomFloatInRange` (+ _returnvalue_y -50.0) (+ _returnvalue_y 50.0)) _returnvalue_z)) "AlwaysSpawn" "MultiplyWithRoot" null "NewEnumerator1" null))
            (`self.K2_DestroyActor`)
            (else
              (`TimelineComponent.PlayFromStart` (`self.GotHit`)))))))))

(fn `Random Mesh`
  (switch `/Game/Assets/SpaceGrabage/E_GrabageType` (`self.GrabageType`)
    (:`NewEnumerator0`
      (`StaticMeshComponent.SetStaticMesh` (`self.Mesh`) (`KismetArrayLibrary.Array_Random` (`self.BigGrabageMeshes`)))
      (`SceneComponent.SetWorldScale3D` (`self.Mesh`) (10.0 10.0 10.0))
      (`PrimitiveComponent.SetMassOverrideInKg` (`self.Mesh`) "None" 100.0 true))
    (:`NewEnumerator1`
      (`StaticMeshComponent.SetStaticMesh` (`self.Mesh`) (`KismetArrayLibrary.Array_Random` (`self.SmallGrabageMeshes`)))
      (`SceneComponent.SetWorldScale3D` (`self.Mesh`) (6.0 6.0 6.0))))
  (set `self.DefaultScale` (`SceneComponent.K2_GetComponentScale` (`self.Mesh`))))

(fn `UserConstructionScript`)