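; BP_GarbageGenerator populates a band of space debris around an Earth-sized radius when play begins.
; It loops over the start count, spawning BP_SpaceGrabage actors in the XY plane using random angles and a square-root-weighted random offset within the band's thickness, beyond the start altitude.
; The construction script draws a debug sphere at the Earth radius, and BeginPlay prints the start altitude after spawning.
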(event `self.ReceiveBeginPlay`
  (bind _garbagespherealtitudestart (`self.GarbagesphereAltitudeStart`))
  (bind _returnvalue (`KismetMathLibrary.RandomFloatInRange` 0.0 (* (`KismetMathLibrary.GetPI`) 2.0)))
  (bind _returnvalue_2 (+ (+ (`self.EarthRadius`) _garbagespherealtitudestart) (* (`self.GarbagesphereThickness`) (`KismetMathLibrary.Sqrt` (`KismetMathLibrary.RandomFloat`)))))
  (for _ (range (+ (`self.GarbageStartCount`) 1))
    (`|SpawnActorFromClass` "/Game/Assets/SpaceGrabage/BP_SpaceGrabage.BP_SpaceGrabage_C" (`KismetMathLibrary.MakeTransform` (`KismetMathLibrary.MakeVector` (* _returnvalue_2 (`KismetMathLibrary.Cos` _returnvalue)) (* _returnvalue_2 (`KismetMathLibrary.Sin` _returnvalue)))) "Undefined" "MultiplyWithRoot" null null))
  (`KismetSystemLibrary.PrintString` (`KismetStringLibrary.Conv_DoubleToString` _garbagespherealtitudestart)))

(fn `UserConstructionScript`
  (`KismetSystemLibrary.DrawDebugSphere` (0.0 0.0 0.0) (`self.EarthRadius`)))