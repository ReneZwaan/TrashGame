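; Space gun actor that fires BP_Projectile from its FireLocation, with a bullet sound at the spawn point.
; Tick runs through a one-second Delay for repeated automatic shots, while the Fire event spawns immediately, bypassing the delay.
; Projectiles spawn at a rotated forward offset and take FireLocation's rotation.
; LimitGunRotAngle clamps GunShoot's yaw around the value stored at BeginPlay, but its only call is unreachable.
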(event `self.ReceiveBeginPlay`
  (bind (_relativerotation_roll _relativerotation_pitch _relativerotation_yaw) (`KismetMathLibrary.BreakRotator` (`SceneComponent.RelativeRotation` (`self.gun_shoot`))))
  (set `self.GunDefaultRotZ` _relativerotation_yaw))

(event `self.ReceiveTick`
  (params (DeltaSeconds :type "Float (single-precision)"))
  (bind _returnvalue (`SceneComponent.K2_GetComponentRotation` (`self.FireLocation`)))
  (bind _returnvalue_2 (+ (`SceneComponent.K2_GetComponentLocation` (`self.FireLocation`)) (`KismetMathLibrary.GreaterGreater_VectorRotator` (`self.ProjectileOffset`) _returnvalue)))
  (`KismetSystemLibrary.Delay` 1.0)
  (`|SpawnActorFromClass` "/Game/Assets/SpaceGun/BP_Projectile.BP_Projectile_C" (`KismetMathLibrary.MakeTransform` _returnvalue_2 _returnvalue) "AlwaysSpawn" "MultiplyWithRoot" null null :!label _label)
  (`GameplayStatics.SpawnSoundAtLocation` "/Game/Assets/Sound/bullet_Cue.bullet_Cue" _returnvalue_2 (struct) 1.0 1.0 0.0 null null))

(event `Fire`
  (goto _label))

(fn `LimitGunRotAngle`
  (bind _gun_shoot (`self.gun_shoot`))
  (bind _returnvalue (+ (`self.GunDefaultRotZ`) 20.0))
  (bind _returnvalue_2 (+ (`self.GunDefaultRotZ`) -20.0))
  (bind (_relativerotation_roll _relativerotation_pitch _relativerotation_yaw) (`KismetMathLibrary.BreakRotator` (`SceneComponent.RelativeRotation` _gun_shoot)))
  (bind (_relativerotation_roll_2 _relativerotation_pitch_2 _relativerotation_yaw_2) (`KismetMathLibrary.BreakRotator` (`SceneComponent.RelativeRotation` (`self.gun_shoot`))))
  (if (not (`KismetMathLibrary.InRange_FloatFloat` _relativerotation_yaw_2 _returnvalue_2 _returnvalue))
    (`SceneComponent.K2_SetRelativeRotation` _gun_shoot (`KismetMathLibrary.MakeRotator` _relativerotation_roll _relativerotation_pitch (`KismetMathLibrary.FClamp` _relativerotation_yaw _returnvalue_2 _returnvalue)) false false))
  (return))

(fn `UserConstructionScript`)