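; Player controller that handles movement input for four players through one controller.
; Each player has its own Enhanced Input move action, and on Started it loops the Players array to find the entry with the matching PlayerIndex.
; That player receives an AddImpulseToTargetPlayer call, with the input axes swapped into world X/Y, scaled by ImpulseStrength, and no vertical impulse.
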(event `EnhancedInput|/Game/Assets/Player/Input/Actions/AI_Move_P1`
  (params (ActionValue :type "Vector2D Structure") (ElapsedSeconds :type "Float (double-precision)") (TriggeredSeconds :type "Float (double-precision)") (InputAction :type "InputAction Object Reference" :default "/Game/Assets/Player/Input/Actions/AI_Move_P1.AI_Move_P1"))
  (bind (_x _y) (`KismetMathLibrary.BreakVector2D` ActionValue))
  (bind _impulsestrength (`self.ImpulseStrength`))
  (:`Started`
    (for _array_element (`self.Players`)
      (if (== (`/Game/Assets/Player/BP_Player.PlayerIndex` _array_element) 0)
        (`/Game/Assets/Player/BP_Player.Add Impulse To Target Player` _array_element (`KismetMathLibrary.MakeVector` (* _y _impulsestrength) (* _x _impulsestrength)))))))

(event `EnhancedInput|/Game/Assets/Player/Input/Actions/AI_Move_P2`
  (params (ActionValue :type "Vector2D Structure") (ElapsedSeconds :type "Float (double-precision)") (TriggeredSeconds :type "Float (double-precision)") (InputAction :type "InputAction Object Reference" :default "/Game/Assets/Player/Input/Actions/AI_Move_P2.AI_Move_P2"))
  (bind (_x _y) (`KismetMathLibrary.BreakVector2D` ActionValue))
  (bind _impulsestrength (`self.ImpulseStrength`))
  (:`Started`
    (for _array_element (`self.Players`)
      (if (== (`/Game/Assets/Player/BP_Player.PlayerIndex` _array_element) 1)
        (`/Game/Assets/Player/BP_Player.Add Impulse To Target Player` _array_element (`KismetMathLibrary.MakeVector` (* _y _impulsestrength) (* _x _impulsestrength)))))))

(event `EnhancedInput|/Game/Assets/Player/Input/Actions/AI_Move_P3`
  (params (ActionValue :type "Vector2D Structure") (ElapsedSeconds :type "Float (double-precision)") (TriggeredSeconds :type "Float (double-precision)") (InputAction :type "InputAction Object Reference" :default "/Game/Assets/Player/Input/Actions/AI_Move_P3.AI_Move_P3"))
  (bind (_x _y) (`KismetMathLibrary.BreakVector2D` ActionValue))
  (bind _impulsestrength (`self.ImpulseStrength`))
  (:`Started`
    (for _array_element (`self.Players`)
      (if (== (`/Game/Assets/Player/BP_Player.PlayerIndex` _array_element) 2)
        (`/Game/Assets/Player/BP_Player.Add Impulse To Target Player` _array_element (`KismetMathLibrary.MakeVector` (* _y _impulsestrength) (* _x _impulsestrength)))))))

(event `EnhancedInput|/Game/Assets/Player/Input/Actions/AI_Move_P4`
  (params (ActionValue :type "Vector2D Structure") (ElapsedSeconds :type "Float (double-precision)") (TriggeredSeconds :type "Float (double-precision)") (InputAction :type "InputAction Object Reference" :default "/Game/Assets/Player/Input/Actions/AI_Move_P4.AI_Move_P4"))
  (bind (_x _y) (`KismetMathLibrary.BreakVector2D` ActionValue))
  (bind _impulsestrength (`self.ImpulseStrength`))
  (:`Started`
    (for _array_element (`self.Players`)
      (if (== (`/Game/Assets/Player/BP_Player.PlayerIndex` _array_element) 3)
        (`/Game/Assets/Player/BP_Player.Add Impulse To Target Player` _array_element (`KismetMathLibrary.MakeVector` (* _y _impulsestrength) (* _x _impulsestrength)))))))

(fn `UserConstructionScript`)