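; BP_PlayerManager sets up four-player local multiplayer when play begins.
; It shuffles the level's PlayerStarts and spawns a BP_Player at each of the first four, passing its index.
; The existing controller possesses the first pawn, and CreatePlayer adds a new local player for each of the others.
; Once all are possessed, it tells BP_Camera to blend the view to its target.
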(event `self.ReceiveBeginPlay`
  (bind _returnvalue (`self.GetTransform` (`|GetArrayItem` (`self.PlayerSpawnPoints`) (`self.SpawnPointIndex`))))
  (bind _outactors (`GameplayStatics.GetAllActorsOfClass` "/Script/Engine.PlayerStart"))
  (bind _output_get (set `self.PlayerSpawnPoints` _outactors))
  (`KismetArrayLibrary.Array_Shuffle` _output_get)
  (for _index (range 4)
    (bind _output_get_2 (set `self.SpawnPointIndex` _index))
    (if (> _index 0)
      (bind _returnvalue_2 (`GameplayStatics.CreatePlayer` -1))
      (bind _returnvalue_3 (`|SpawnActorFromClass` "/Game/Assets/Player/BP_Player.BP_Player_C" _returnvalue "Undefined" "MultiplyWithRoot" null (`self.SpawnPointIndex`) null))
      (`Controller.Possess` _returnvalue_2 _returnvalue_3)
      (else
        (bind _returnvalue_4 (`|SpawnActorFromClass` "/Game/Assets/Player/BP_Player.BP_Player_C" _returnvalue "Undefined" "MultiplyWithRoot" null (`self.SpawnPointIndex`) null))
        (`Controller.Possess` (`GameplayStatics.GetPlayerController` 0) _returnvalue_4))))
  (bind _returnvalue_5 (`GameplayStatics.GetActorOfClass` "/Game/Assets/Player/BP_Camera.BP_Camera_C"))
  (`/Game/Assets/Player/BP_Camera.BlendCameraToTarget` _returnvalue_5))

(fn `UserConstructionScript`)