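; BP_Player is a player pawn that shows a "P" number label built from its PlayerIndex.
; On possession it sets the label, adds the default Enhanced Input mapping context and registers itself in the Players list of the first BP_PlayerController found.
; It caches BP_Camera at BeginPlay and exposes a function that applies an impulse to its capsule.
; Escape quits the game; Tick and capsule overlap are empty.
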(event `self.ReceiveBeginPlay`
  (bind _returnvalue (`GameplayStatics.GetActorOfClass` "/Game/Assets/Player/BP_Camera.BP_Camera_C"))
  (set `self.MainCamera` _returnvalue))

(event `self.ReceivePossessed`
  (params (NewController :type "Controller Object Reference"))
  (`TextRenderComponent.K2_SetText` (`self.TextRender`) (`KismetTextLibrary.Conv_StringToText` (`KismetStringLibrary.Concat_StrStr` "P" (`KismetStringLibrary.Conv_IntToString` (+ (`self.PlayerIndex`) 1)))))
  (bind _asplayer_controller (cast `PlayerController` (`self.GetController`)))
  (bind _returnvalue (pcsubsystem `EnhancedInputLocalPlayerSubsystem` _asplayer_controller))
  (`/Engine/EditorBlueprintResources/StandardMacros.IsValid` _returnvalue
    (:`Is Valid`
      (`EnhancedInputSubsystemInterface.AddMappingContext` _returnvalue "/Game/Assets/Player/Input/IMC_Default.IMC_Default" 0 (struct))
      (bind _outactors (`GameplayStatics.GetAllActorsOfClass` "/Game/Assets/Player/BP_PlayerController.BP_PlayerController_C"))
      (`KismetArrayLibrary.Array_AddUnique` (`/Game/Assets/Player/BP_PlayerController.Players` (`|GetArrayItem` _outactors)) self))))

(event `Key|Escape`
  (params (Key :type "Key Structure"))
  (:`Pressed`
    (`KismetSystemLibrary.QuitGame` null "Quit")))

(event `self.ReceiveTick`
  (params (DeltaSeconds :type "Float (single-precision)")))

(event `self.Capsule.OnComponentBeginOverlap`
  (params (OverlappedComponent :type "PrimitiveComponent Object Reference") (OtherActor :type "Actor Object Reference") (OtherComp :type "PrimitiveComponent Object Reference") (OtherBodyIndex :type Integer) (bFromSweep :type Boolean) (SweepResult :type "HitResult Structure (by ref)")))

(fn `Add Impulse To Target Player`
  (params (Impulse :type "Vector Structure"))
  (`PrimitiveComponent.AddImpulse` (`self.Capsule`) Impulse "None" false))

(fn `UserConstructionScript`)