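; BP_Sea is a sea actor that reacts to objects entering its Sphere collision, including garbage bullets.
; On any overlap, it casts its three Fish child actors to BP_Fish in sequence and calls FishFunction on each.
; If the overlapping actor is a BP_BulletGrabage, it then destroys it and prints a debug message.
; A failed fish cast halts the chain, skipping later fish and the bullet cleanup.
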(event `self.ReceiveBeginPlay`)

(event `self.Sphere.OnComponentBeginOverlap`
  (params (OverlappedComponent :type "PrimitiveComponent Object Reference") (OtherActor :type "Actor Object Reference") (OtherComp :type "PrimitiveComponent Object Reference") (OtherBodyIndex :type Integer) (bFromSweep :type Boolean) (SweepResult :type "HitResult Structure (by ref)"))
  (bind _asbp_fish (cast `/Game/Assets/Sea/BP_Fish` (`ChildActorComponent.ChildActor` (`self.Fish`))))
  (bind _output_get (set `self.As BP Fish` _asbp_fish))
  (`/Game/Assets/Sea/BP_Fish.FishFunction` _output_get)
  (bind _asbp_fish_2 (cast `/Game/Assets/Sea/BP_Fish` (`ChildActorComponent.ChildActor` (`self.Fish1`))))
  (bind _output_get_2 (set `self.As BP Fish` _asbp_fish_2))
  (`/Game/Assets/Sea/BP_Fish.FishFunction` _output_get_2)
  (bind _asbp_fish_3 (cast `/Game/Assets/Sea/BP_Fish` (`ChildActorComponent.ChildActor` (`self.Fish2`))))
  (bind _output_get_3 (set `self.As BP Fish` _asbp_fish_3))
  (`/Game/Assets/Sea/BP_Fish.FishFunction` _output_get_3)
  (bind _asbp_bullet_grabage (cast `/Game/Assets/BulletGrabage/BP_BulletGrabage` OtherActor))
  (`self.K2_DestroyActor` _asbp_bullet_grabage)
  (`KismetSystemLibrary.PrintString` "Sea Hited"))

(fn `UserConstructionScript`)