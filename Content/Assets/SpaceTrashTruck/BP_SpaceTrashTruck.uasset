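; A physics-driven space garbage truck that orbits Earth, steered by in-world BP_Button child actors for left, right, eat and poop.
; Left and right apply sideways forces with thruster effects, and eat drives the mouth controller.
; Pooping spends ShitCount to spawn garbage bullets toward Earth and push the ship outward against a constant gravity pull.
; Tick clamps distance from Earth's center to an altitude band and caps speed.
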(event `CloseMouthEvent`
  (params (Type :type "/Game/Assets/Button/E_ButtonType Enum" :default "NewEnumerator0"))
  (bind _asbp_mouth_controller (cast `/Game/Assets/SpaceTrashTruck/BP_MouthController` (`ChildActorComponent.ChildActor` (`self.BP_MouthController`))))
  (`/Game/Assets/SpaceTrashTruck/BP_MouthController.CloseMouthEvent` _asbp_mouth_controller "NewEnumerator4"))

(event `OpenMouthEvent`
  (params (Type :type "/Game/Assets/Button/E_ButtonType Enum" :default "NewEnumerator0"))
  (bind _asbp_mouth_controller (cast `/Game/Assets/SpaceTrashTruck/BP_MouthController` (`ChildActorComponent.ChildActor` (`self.BP_MouthController`))))
  (`/Game/Assets/SpaceTrashTruck/BP_MouthController.OpenMouthEvent` _asbp_mouth_controller "NewEnumerator4"))

(event `self.ReceiveBeginPlay`
  (bind _asbp_button (cast `/Game/Assets/Button/BP_Button` (`ChildActorComponent.ChildActor` (`self.Button_Eat`))))
  (set `/Game/Assets/Button/BP_Button.ButtonType` "NewEnumerator4" _asbp_button)
  (add `/Game/Assets/Button/BP_Button.OnTriggerButton` _asbp_button (delegate `CloseMouthEvent`))
  (add `/Game/Assets/Button/BP_Button.UnTriggerButton` _asbp_button (delegate `OpenMouthEvent`))
  (bind _asbp_button_2 (cast `/Game/Assets/Button/BP_Button` (`ChildActorComponent.ChildActor` (`self.Button_Shit`))))
  (set `/Game/Assets/Button/BP_Button.ButtonType` "NewEnumerator1" _asbp_button_2)
  (add `/Game/Assets/Button/BP_Button.OnTriggerButton` _asbp_button_2 (delegate `CustomEvent`))
  (add `/Game/Assets/Button/BP_Button.UnTriggerButton` _asbp_button_2 (delegate `CustomEvent_0`))
  (bind _asbp_button_3 (cast `/Game/Assets/Button/BP_Button` (`ChildActorComponent.ChildActor` (`self.Button_GoLeft`))))
  (set `/Game/Assets/Button/BP_Button.ButtonType` "NewEnumerator2" _asbp_button_3)
  (add `/Game/Assets/Button/BP_Button.OnTriggerButton` _asbp_button_3 (delegate `MoveLeftEvent`))
  (add `/Game/Assets/Button/BP_Button.UnTriggerButton` _asbp_button_3 (delegate `UnMoveLeftEvent`))
  (`ActorComponent.Deactivate` (`self.Fire_Right`))
  (bind _asbp_button_4 (cast `/Game/Assets/Button/BP_Button` (`ChildActorComponent.ChildActor` (`self.Button_GoRight`))))
  (set `/Game/Assets/Button/BP_Button.ButtonType` "NewEnumerator3" _asbp_button_4)
  (add `/Game/Assets/Button/BP_Button.OnTriggerButton` _asbp_button_4 (delegate `MoveRightEvent`))
  (add `/Game/Assets/Button/BP_Button.UnTriggerButton` _asbp_button_4 (delegate `UnMoveRightEvent`))
  (`ActorComponent.Deactivate` (`self.Fire_left`)))

(event `CustomEvent`
  (params (Type :type "/Game/Assets/Button/E_ButtonType Enum" :default "NewEnumerator0"))
  (switch `/Game/Assets/Button/E_ButtonType` Type
    (:`NewEnumerator1`
      (set `self.WannaShit` true))))

(event `CustomEvent_0`
  (params (Type :type "/Game/Assets/Button/E_ButtonType Enum" :default "NewEnumerator0"))
  (switch `/Game/Assets/Button/E_ButtonType` Type
    (:`NewEnumerator1`
      (set `self.WannaShit` false))))

(event `UnMoveLeftEvent`
  (params (Type :type "/Game/Assets/Button/E_ButtonType Enum" :default "NewEnumerator0"))
  (switch `/Game/Assets/Button/E_ButtonType` Type
    (:`NewEnumerator2`
      (set `self.MovingLeft` false)
      (`ActorComponent.Deactivate` (`self.Fire_Right`)))))

(event `UnMoveRightEvent`
  (params (Type :type "/Game/Assets/Button/E_ButtonType Enum" :default "NewEnumerator0"))
  (set `self.MovingRight` false)
  (`ActorComponent.Deactivate` (`self.Fire_left`)))

(event `MoveLeftEvent`
  (params (Type :type "/Game/Assets/Button/E_ButtonType Enum" :default "NewEnumerator0"))
  (switch `/Game/Assets/Button/E_ButtonType` Type
    (:`NewEnumerator2`
      (set `self.MovingLeft` true)
      (`ActorComponent.Activate` (`self.Fire_Right`) false))))

(event `MoveRightEvent`
  (params (Type :type "/Game/Assets/Button/E_ButtonType Enum" :default "NewEnumerator0"))
  (set `self.MovingRight` true)
  (`ActorComponent.Activate` (`self.Fire_left`) false))

(event `self.ReceiveTick`
  (params (DeltaSeconds :type "Float (single-precision)"))
  (bind _space_ship (`self.space_ship`))
  (bind _returnvalue (`SceneComponent.K2_GetComponentLocation` (`self.Scene`)))
  (bind _returnvalue_2 (* (`self.EarthSize`) (/ (`self.DistanceFromEarthCenter`) 100.0)))
  (bind _returnvalue_3 (- (`SceneComponent.K2_GetComponentLocation` _space_ship) _returnvalue))
  (bind _returnvalue_4 (`KismetMathLibrary.VSize` _returnvalue_3))
  (bind _returnvalue_5 (+ _returnvalue_2 (`self.FlyingMarginLow`)))
  (bind _returnvalue_6 (+ _returnvalue_2 (`self.FlyingMarginHigh`)))
  (`|ExecutionSequence`
    (:`then_0`
      (bind _output_get (set `self.IsShitting` (and (> (`self.ShitCount`) 0) (`self.WannaShit`))))
      (if _output_get
        (`KismetSystemLibrary.Delay` 0.2)
        (`/Engine/EditorBlueprintResources/StandardMacros.DecrementInt` (`self.ShitCount`)
          (:`  `
            (`self.Move To Space` (`self.PoopDirectionalStrength`))
            (`|SpawnActorFromClass` "/Game/Assets/BulletGrabage/BP_BulletGrabage.BP_BulletGrabage_C" (`SceneComponent.K2_GetComponentToWorld` (`self.Earth Direction`)) "Undefined" "MultiplyWithRoot" null null)))
        (else
          (`self.Move To Earth` (* (`self.BaseGravStrengt`) DeltaSeconds)))))
    (:`then_1`
      (if (`self.MovingLeft`)
        (`self.MoveLeft` (`self.DirectionalStrength`))))
    (:`then_2`
      (if (`self.MovingRight`)
        (`self.MoveRight` (`self.DirectionalStrength`))))
    (:`then_3`
      (if (`self.IsShitting`)
        (`self.Move To Space` (* (`self.PoopDirectionalStrength`) DeltaSeconds))))
    (:`then_4`
      (if (or (< _returnvalue_4 _returnvalue_5) (> _returnvalue_4 _returnvalue_6))
        (`SceneComponent.K2_SetWorldLocation` _space_ship (+ _returnvalue (`KismetMathLibrary.ClampVectorSize` _returnvalue_3 _returnvalue_5 _returnvalue_6)) false false)
        (`PrimitiveComponent.SetPhysicsLinearVelocity` _space_ship (0.0 0.0 0.0) false "None")))
    (:`then_5`
      (bind _returnvalue_7 (`PrimitiveComponent.GetPhysicsLinearVelocity` _space_ship "None"))
      (if (> (`KismetMathLibrary.VSize` _returnvalue_7) 300.0)
        (`PrimitiveComponent.SetPhysicsLinearVelocity` _space_ship (`KismetMathLibrary.ClampVectorSize` _returnvalue_7 0.0 300.0) false "None")))))

(event `MoveLeft`
  (params (B :type "Float (double-precision)"))
  ;[1 1 1] Space ship controll functions
  (`PrimitiveComponent.AddForce` (`self.space_ship`) (* (`KismetMathLibrary.Quat_VectorForward` (`KismetMathLibrary.Conv_RotatorToQuaternion` (`SceneComponent.K2_GetComponentRotation` (`self.DirectionLeft`)))) B) "None" true))

(event `MoveRight`
  (params (B :type "Float (double-precision)"))
  ;[1 1 1] Space ship controll functions
  (`PrimitiveComponent.AddForce` (`self.space_ship`) (* (`KismetMathLibrary.Quat_VectorForward` (`KismetMathLibrary.Conv_RotatorToQuaternion` (`SceneComponent.K2_GetComponentRotation` (`self.DirectionRight`)))) B) "None" true))

(event `Move To Earth`
  (params (Strength :type "Float (double-precision)"))
  ;[1 1 1] Space ship controll functions
  (`PrimitiveComponent.AddForce` (`self.space_ship`) (* (`KismetMathLibrary.Quat_VectorForward` (`KismetMathLibrary.Conv_RotatorToQuaternion` (`SceneComponent.K2_GetComponentRotation` (`self.Earth Direction`)))) Strength) "None" true))

(event `Move To Space`
  (params (Strength :type "Float (double-precision)"))
  ;[1 1 1] Space ship controll functions
  (`PrimitiveComponent.AddForce` (`self.space_ship`) (* (`KismetMathLibrary.Normal` (- (`SceneComponent.K2_GetComponentLocation` (`self.space_ship`)) (`SceneComponent.K2_GetComponentLocation` (`self.Scene`)))) Strength) "None" true))

(event `Key|D`
  (params (Key :type "Key Structure"))
  (:`Pressed`
    (`self.MoveRight` 0.0)))

(event `Key|A`
  (params (Key :type "Key Structure"))
  (:`Pressed`
    (`self.MoveLeft` 0.0)))

(event `Key|W`
  (params (Key :type "Key Structure"))
  (:`Pressed`
    (set `self.WannaShit` true))
  (:`Released`
    (set `self.WannaShit` false)))

(fn `UserConstructionScript`
  (bind _earth (`self.Earth`))
  (`SceneComponent.K2_SetWorldLocation` (`self.Scene`) (`self.K2_GetActorLocation` _earth) false false)
  (`SceneComponent.K2_AddLocalOffset` (`self.space_ship`) (`KismetMathLibrary.MakeVector` (* (/ (.x (`.BoxExtent` (`self.GetActorBounds` _earth false false))) 100.0) (`self.DistanceFromEarthCenter`))) false false))