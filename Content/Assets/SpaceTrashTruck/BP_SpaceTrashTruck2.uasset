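; Player-driven space trash truck pawn or actor that hovers around Earth, using velocity-change impulses on the SpaceShip component.
; Construction centers the Scene on Earth and offsets the ship by a distance scaled from Earth's bounds.
; Tick applies gravity toward Earth and, once Shit is triggered, spends ShitCount on delayed, random-strength boosts toward space.
; Test keys A and D push sideways along direction components; W triggers Shit.
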(event `self.ReceiveBeginPlay`)

(event `self.ReceiveTick`
  (params (DeltaSeconds :type "Float (single-precision)"))
  (`self.Move To Earth` (* (`self.BaseGravStrengt`) DeltaSeconds))
  (if (and (> (`self.ShitCount`) 0) (`self.IsShitting`))
    (`KismetSystemLibrary.Delay` 0.2)
    (`self.Move To Space` (`KismetMathLibrary.RandomFloatInRange` 500.0 1500.0))
    (`/Engine/EditorBlueprintResources/StandardMacros.DecrementInt` (`self.ShitCount`))))

(event `Shit`
  (set `self.IsShitting` true))

(event `MoveLeft`
  ;[1 1 1] Space ship controll functions
  (`PrimitiveComponent.AddImpulse` (`self.space_ship`) (* (`SceneComponent.K2_GetComponentRotation` (`self.DirectionLeft`)) (`self.DirectionalStrength`)) "None" true))

(event `MoveRight`
  ;[1 1 1] Space ship controll functions
  (`PrimitiveComponent.AddImpulse` (`self.space_ship`) (* (`SceneComponent.K2_GetComponentRotation` (`self.DirectionRight`)) (`self.DirectionalStrength`)) "None" true))

(event `Move To Earth`
  (params (Strength :type "Float (double-precision)"))
  ;[1 1 1] Space ship controll functions
  (`PrimitiveComponent.AddImpulse` (`self.space_ship`) (* (`SceneComponent.K2_GetComponentRotation` (`self.Earth Direction`)) Strength) "None" true))

(event `Move To Space`
  (params (Strength :type "Float (double-precision)"))
  ;[1 1 1] Space ship controll functions
  (`PrimitiveComponent.AddImpulse` (`self.space_ship`) (* (`SceneComponent.K2_GetComponentRotation` (`self.Space Direction`)) Strength) "None" true))

(event `Key|D`
  (params (Key :type "Key Structure"))
  (:`Pressed`
    (`self.MoveRight`)))

(event `Key|A`
  (params (Key :type "Key Structure"))
  (:`Pressed`
    (`self.MoveLeft`)))

(event `Key|W`
  (params (Key :type "Key Structure"))
  (:`Pressed`
    (`self.Shit`)))

(fn `UserConstructionScript`
  (bind _earth (`self.Earth`))
  (`SceneComponent.K2_SetWorldLocation` (`self.Scene`) (`self.K2_GetActorLocation` _earth) false false)
  (`SceneComponent.K2_AddLocalOffset` (`self.space_ship`) (`KismetMathLibrary.MakeVector` (* (/ (.x (`.BoxExtent` (`self.GetActorBounds` _earth false false))) 100.0) (`self.DistanceFromEarthCenter`))) false false))