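; Mouth of the space trash truck that chomps and eats space garbage when a child-actor button is pressed.
; Button events keep a close timer topped up, and while it runs the mouth alternates shut and open every half second.
; Tick swings the upper and lower pivots at constant speed.
; While flagged closed, it destroys garbage overlapping its box, plays an eat sound and increases the truck's ShitCount.
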(event `self.ReceiveBeginPlay`
  (bind _asbp_button (cast `/Game/Assets/Button/BP_Button` (`ChildActorComponent.ChildActor` (`self.BP_Button`))))
  (add `/Game/Assets/Button/BP_Button.OnTriggerButton` _asbp_button (delegate `CloseMouthEvent`))
  (add `/Game/Assets/Button/BP_Button.UnTriggerButton` _asbp_button (delegate `OpenMouthEvent`)))

(event `CloseMouthEvent`
  (params (Type :type "/Game/Assets/Button/E_ButtonType Enum" :default "NewEnumerator0"))
  (set `self.MouthButtonPressed` true))

(event `OpenMouthEvent`
  (params (Type :type "/Game/Assets/Button/E_ButtonType Enum" :default "NewEnumerator0"))
  (set `self.MouthButtonPressed` false))

(event `self.ReceiveTick`
  (params (DeltaSeconds :type "Float (single-precision)"))
  (bind _downpivot (`self.DownPivot`))
  (bind _mouthspeed (`self.MouthSpeed`))
  (bind _uppivot (`self.UpPivot`))
  (if (`self.MouthButtonPressed`)
    (set `self.MouthCloseTimer` (`self.MouthCloseTime`))
    (else
      (set `self.MouthCloseTimer` (- (`self.MouthCloseTimer`) DeltaSeconds))))
  (if (> (`self.MouthCloseTimer`) 0.0)
    (bind _output_get (set `self.TimeAcc` (+ (`self.TimeAcc`) DeltaSeconds)))
    (set `self.MouthClosed` (== (mod (`.ReturnValue` (`KismetMathLibrary.FMod` _output_get 0.5)) 2) 0))
    (else
      (set `self.MouthClosed` false)
      (set `self.TimeAcc` 0.0)))
  (if (`self.MouthClosed`)
    (set `self.WantedRot` (struct))
    (else
      (set `self.WantedRot` (`KismetMathLibrary.MakeRotator` 0.0 0.0 (* (`self.MouthOpenAngle`) -1.0)))))
  (`SceneComponent.K2_SetRelativeRotation` _downpivot (`KismetMathLibrary.RInterpTo_Constant` (`SceneComponent.RelativeRotation` _downpivot) (`self.WantedRot`) DeltaSeconds _mouthspeed) false false)
  (if (`self.MouthClosed`)
    (set `self.WantedRot` (struct))
    (else
      (set `self.WantedRot` (`KismetMathLibrary.MakeRotator` 0.0 0.0 (`self.MouthOpenAngle`)))))
  (`SceneComponent.K2_SetRelativeRotation` _uppivot (`KismetMathLibrary.RInterpTo_Constant` (`SceneComponent.RelativeRotation` _uppivot) (`self.WantedRot`) DeltaSeconds _mouthspeed) false false)
  (if (`self.MouthClosed`)
    (for _array_element (`PrimitiveComponent.GetOverlappingActors` (`self.Box`) null)
      (bind _asbp_space_grabage (cast `/Game/Assets/SpaceGrabage/BP_SpaceGrabage` _array_element))
      (`GameplayStatics.SpawnSoundAtLocation` "/Game/Assets/Sound/eat_Cue.eat_Cue" (`self.K2_GetActorLocation`) (struct) 1.0 1.0 0.0 null null)
      (`self.K2_DestroyActor` _asbp_space_grabage)
      (bind _returnvalue (`GameplayStatics.GetActorOfClass` "/Game/Assets/SpaceTrashTruck/BP_SpaceTrashTruck.BP_SpaceTrashTruck_C"))
      (set `/Game/Assets/SpaceTrashTruck/BP_SpaceTrashTruck.ShitCount` (+ (`/Game/Assets/SpaceTrashTruck/BP_SpaceTrashTruck.ShitCount` _returnvalue) 3) _returnvalue))))

(fn `UserConstructionScript`)